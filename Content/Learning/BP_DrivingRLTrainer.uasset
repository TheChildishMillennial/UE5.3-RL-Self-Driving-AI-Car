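; Learning Agents reinforcement learning trainer that teaches sports car pawns to drive along the track spline found at BeginPlay.
; A spline helper supplies each car's nearest track point and its velocity along the spline.
; These drive a speed reward, an off-track penalty and, at a wider distance threshold, an off-track completion.
; Episode resets move each car to a random point on the spline.
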(event `self.ReceiveBeginPlay`
  (bind _returnvalue (`GameplayStatics.GetActorOfClass` "/Game/Learning/BP_SportCarTrackSpline.BP_SportCarTrackSpline_C"))
  (set `self.TrackSpline` (`/Game/Learning/BP_SportCarTrackSpline.Spline` _returnvalue)))

(event `self.SetupRewards`
  (`|ExecutionSequence`
    (:`then_0`
      (bind _returnvalue (`PlanarPositionDifferencePenalty.AddPlanarPositionDifferencePenalty` null "OffTrackPenalty" 1.0 100.0 800.0))
      (set `self.OffTrackPenalty` _returnvalue))
    (:`then_1`
      (bind _returnvalue_2 (`ScalarVelocityReward.AddScalarVelocityReward` null "SpeedReward" 0.1))
      (set `self.VelocityAlongTrackReward` _returnvalue_2))
    (:`then_2`
      (bind _returnvalue_3 (`SplineComponentHelper.AddSplineComponentHelper` null "SplineComponentRewardHelper"))
      (set `self.SplineComponentRewardHelper` _returnvalue_3))))

(event `self.SetRewards`
  (params (AgentIds :type "Array of Integer (by ref)"))
  (for _array_element AgentIds
    (`|ExecutionSequence`
      (:`then_0`
        (bind _returnvalue (`self.GetAgent` _array_element "/Game/VehicleTemplate/Blueprints/SportsCar/BP_SportsCar_Pawn.BP_SportsCar_Pawn_C"))
        (bind _returnvalue_2 (`Actor.K2_GetActorLocation` _returnvalue))
        (bind _returnvalue_3 (`SplineComponentHelper.GetNearestPositionOnSpline` (`self.SplineComponentRewardHelper`) _array_element (`self.TrackSpline`) _returnvalue_2 "World"))
        (`PlanarPositionDifferencePenalty.SetPlanarPositionDifferencePenalty` (`self.OffTrackPenalty`) _array_element _returnvalue_3 _returnvalue_2))
      (:`then_1`
        (bind _returnvalue_4 (`SplineComponentHelper.GetVelocityAlongSpline` (`self.SplineComponentRewardHelper`) _array_element (`self.TrackSpline`) _returnvalue_2 (`Actor.GetVelocity` _returnvalue) 10.0 "World"))
        (`ScalarVelocityReward.SetScalarVelocityReward` (`self.VelocityAlongTrackReward`) _array_element _returnvalue_4)))))

(event `self.SetupCompletions`
  (bind _returnvalue (`PlanarPositionDifferenceCompletion.AddPlanarPositionDifferenceCompletion` null "OffTrackCompletion" 1200.0))
  (set `self.OffTrackTermination` _returnvalue))

(event `self.SetCompletions`
  (params (AgentIds :type "Array of Integer (by ref)"))
  (for _array_element AgentIds
    (bind _returnvalue (`Actor.K2_GetActorLocation` (`self.GetAgent` _array_element "/Game/VehicleTemplate/Blueprints/SportsCar/BP_SportsCar_Pawn.BP_SportsCar_Pawn_C")))
    (bind _returnvalue_2 (`SplineComponentHelper.GetNearestPositionOnSpline` (`self.SplineComponentRewardHelper`) _array_element (`self.TrackSpline`) _returnvalue "World"))
    (`PlanarPositionDifferenceCompletion.SetPlanarPositionDifferenceCompletion` (`self.OffTrackTermination`) _array_element _returnvalue_2 _returnvalue)))

(event `self.ResetEpisodes`
  (params (AgentIds :type "Array of Integer (by ref)"))
  (for _array_element AgentIds
    (`/Game/VehicleTemplate/Blueprints/SportsCar/BP_SportsCar_Pawn.Reset to Random Point on Spline` (`self.GetAgent` _array_element "/Game/VehicleTemplate/Blueprints/SportsCar/BP_SportsCar_Pawn.BP_SportsCar_Pawn_C") (`self.TrackSpline`))))