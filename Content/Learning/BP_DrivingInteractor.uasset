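; Learning Agents interactor that defines what sports car agents observe and how they drive along a spline track.
; Observations use a spline helper on the track found in the level: nearest track position and direction relative to the car, lap progress as an angle, and car-relative velocity.
; Two float actions drive each car's vehicle movement component: one signed value split into throttle or brake, the other for steering.
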(event `self.SetupObservations`
  (`|ExecutionSequence`
    (:`then_0`
      (bind _returnvalue (`PlanarPositionObservation.AddPlanarPositionObservation` null "TrackPositionObservation"))
      (set `self.TrackPositionObservation` _returnvalue)
      (bind _returnvalue_2 (`PlanarDirectionObservation.AddPlanarDirectionObservation` null "TrackDirectionObservation"))
      (set `self.TrackDirectionObservation` _returnvalue_2))
    (:`then_1`
      (bind _returnvalue_3 (`AngleObservation.AddAngleObservation` null "TrackGlobalPositionObservation"))
      (set `self.TrackGlobalPositionObservation` _returnvalue_3)
      (bind _returnvalue_4 (`PlanarVelocityObservation.AddPlanarVelocityObservation` null "CarVelocityObservation"))
      (set `self.CarVelocityObservation` _returnvalue_4))
    (:`then_2`
      (bind _returnvalue_5 (`SplineComponentHelper.AddSplineComponentHelper` null "SplineComponentHelper"))
      (set `self.SplineComponentHelper` _returnvalue_5)
      (bind _returnvalue_6 (`GameplayStatics.GetActorOfClass` "/Game/Learning/BP_SportCarTrackSpline.BP_SportCarTrackSpline_C"))
      (set `self.TrackSpline` (`/Game/Learning/BP_SportCarTrackSpline.Spline` _returnvalue_6)))))

(event `self.SetObservations`
  (params (AgentIds :type "Array of Integer (by ref)"))
  (for _array_element AgentIds
    (bind _returnvalue (`self.GetAgent` _array_element "/Game/VehicleTemplate/Blueprints/SportsCar/BP_SportsCar_Pawn.BP_SportsCar_Pawn_C"))
    (bind _returnvalue_2 (`Actor.K2_GetActorLocation` _returnvalue))
    (bind _returnvalue_3 (`SplineComponentHelper.GetDistanceAlongSplineAtPosition` (`self.SplineComponentHelper`) _array_element (`self.TrackSpline`) _returnvalue_2 "World"))
    (`|ExecutionSequence`
      (:`then_0`
        (bind _returnvalue_4 (`SplineComponentHelper.GetPositionAtDistanceAlongSpline` (`self.SplineComponentHelper`) _array_element (`self.TrackSpline`) _returnvalue_3 "World"))
        (bind _returnvalue_5 (`Actor.K2_GetActorRotation` _returnvalue))
        (`PlanarPositionObservation.SetPlanarPositionObservation` (`self.TrackPositionObservation`) _array_element _returnvalue_4 _returnvalue_2 _returnvalue_5))
      (:`then_1`
        (bind _returnvalue_6 (`SplineComponentHelper.GetDirectionAtDistanceAlongSpline` (`self.SplineComponentHelper`) _array_element (`self.TrackSpline`) _returnvalue_3 "World"))
        (`PlanarDirectionObservation.SetPlanarDirectionObservation` (`self.TrackDirectionObservation`) _array_element _returnvalue_6 _returnvalue_5))
      (:`then_2`
        (bind _returnvalue_7 (`SplineComponentHelper.GetProportionAlongSplineAsAngle` (`self.SplineComponentHelper`) _array_element (`self.TrackSpline`) _returnvalue_3))
        (`AngleObservation.SetAngleObservation` (`self.TrackGlobalPositionObservation`) _array_element _returnvalue_7 0.0))
      (:`then_3`
        (`PlanarVelocityObservation.SetPlanarVelocityObservation` (`self.CarVelocityObservation`) _array_element (`Actor.GetVelocity` _returnvalue) _returnvalue_5)))))

(event `self.SetupActions`
  (`|ExecutionSequence`
    (:`then_0`
      (bind _returnvalue (`FloatAction.AddFloatAction` null "ThrottleBrakeAction"))
      (set `self.ThrottleBrakeAction` _returnvalue))
    (:`then_1`
      (bind _returnvalue_2 (`FloatAction.AddFloatAction` null "SteeringAction"))
      (set `self.SteeringAction` _returnvalue_2))))

(event `self.GetActions`
  (params (AgentIds :type "Array of Integer (by ref)"))
  (for _array_element AgentIds
    (`|ExecutionSequence`
      (:`then_0`
        (bind _returnvalue (`FloatAction.GetFloatAction` (`self.ThrottleBrakeAction`) _array_element))
        (if (> _returnvalue 0.0)
          (bind _returnvalue_2 (`self.GetAgent` _array_element "/Game/VehicleTemplate/Blueprints/SportsCar/BP_SportsCar_Pawn.BP_SportsCar_Pawn_C"))
          (bind _vehiclemovementcomponent (`WheeledVehiclePawn.VehicleMovementComponent` _returnvalue_2))
          (`ChaosVehicleMovementComponent.SetThrottleInput` _vehiclemovementcomponent _returnvalue)
          (`ChaosVehicleMovementComponent.SetBrakeInput` _vehiclemovementcomponent 0.0)
          (else
            (`ChaosVehicleMovementComponent.SetThrottleInput` _vehiclemovementcomponent 0.0)
            (`ChaosVehicleMovementComponent.SetBrakeInput` _vehiclemovementcomponent (- 0.0 _returnvalue)))))
      (:`then_1`
        (bind _returnvalue_3 (`FloatAction.GetFloatAction` (`self.SteeringAction`) _array_element))
        (`ChaosVehicleMovementComponent.SetSteeringInput` (`WheeledVehiclePawn.VehicleMovementComponent` _returnvalue_2) _returnvalue_3)))))